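; Main pawn of a Doom-style WAD launcher app that starts an external source port with the chosen game files.
; BeginPlay shows the main screen in UI-only input, disables world rendering, caps frame rate and enables idling when unfocused.
; LaunchGame builds IWAD, PWAD and extra arguments, then spawns a detached process through a Victory plugin node.
; It then either quits the launcher or clears the argument list.
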(event Custom|Launch%20Game
  (params (SourcePortPath :type String) (IWAD_Path :type String) (PWAD_Path :type Array%20of%20Strings) (AdditionalArgs :type String))
  (Utilities|FlowControl|Sequence
    (:then_0
      (Utilities|Array|Insert (Variables|Default|GetCommandLineArgs) (Class|VictoryBPFunctionLibrary|AppendMultiple "-iwad " "\"" IWAD_Path "\" ")))
    (:then_1
      (for _array_element PWAD_Path
        (Variables|Default|SetPWAD_PathLine (Utilities|String|Append (Variables|Default|GetPWAD_PathLine) "\"" _array_element "\" ")))
      (Utilities|Array|Insert (Variables|Default|GetCommandLineArgs) (Utilities|String|Append "-file " (Variables|Default|GetPWAD_PathLine)) 1))
    (:then_2
      (Utilities|Array|Insert (Variables|Default|GetCommandLineArgs) AdditionalArgs 2))
    (:then_3
      (Class|VictoryBPFunctionLibrary|VictoryCreateProc SourcePortPath (Variables|Default|GetCommandLineArgs) true false)
      (if (Variables|Default|GetQuitLauncher)
        (Game|QuitGame 0 "Quit" false)
        (else
          (Utilities|Array|Clear (Variables|Default|GetCommandLineArgs)))))))

(event EventBeginPlay
  (bind _returnvalue (Game|GetPlayerController 0))
  (bind _returnvalue_2 (UserInterface|CreateWidget "/Game/TODD/Widget/UI_MainScreen.UI_MainScreen_C" 0 0))
  (UserInterface|Viewport|AddtoViewport _returnvalue_2 0)
  (Input|SetInputModeUIOnly _returnvalue _returnvalue_2 "DoNotLock")
  (Variables|/Script/Engine.PlayerController|SetbShowMouseCursor _returnvalue true)
  (Class|VictoryBPFunctionLibrary|ViewportEnableWorldRendering _returnvalue false)
  (Class|VictoryBPFunctionLibrary|GraphicsSettingsSetFrameRateCap 1.2e+02)
  (Development|ExecuteConsoleCommand "t.IdleWhenNotForeground 1" 0))

(event Collision|EventActorBeginOverlap
  (params (OtherActor :type Actor%20Object%20Reference)))

(event EventTick
  (params (DeltaSeconds :type Float%20%28single-precision%29)))

(fn ConstructionScript)